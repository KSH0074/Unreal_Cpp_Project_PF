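; AI controller for the boss monster, which starts its behavior tree after an intro animation.
; On possessing a BossMonster, it waits briefly, plays the level-start montage, and runs BT_Boss when that montage completes.
; It stores the player pawn in the blackboard at BeginPlay and updates the boss-to-player distance there every tick for the tree to read.
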(event EventBeginPlay
  (AI|Components|Blackboard|SetValueasObject (Variables|Default|GetBlackboard1) (Variables|Default|GetMainPlayer) (Game|Player|GetPlayerPawn 0)))

(event EventTick
  (params (DeltaSeconds :type Float%20%28single-precision%29))
  (AI|Components|Blackboard|SetValueasFloat (Variables|Default|GetBlackboard1) (Variables|Default|GetDistance) (Math|Vector|Distance(Vector) (Transformation|GetActorLocation (stale EventPossess PossessedPawn)) (Transformation|GetActorLocation (Game|Player|GetPlayerPawn 0)))))

(event EventPossess
  (params (PossessedPawn :type Pawn%20Object%20Reference))
  (bind _asboss_monster (Utilities|Casting|CastToBossMonster PossessedPawn))
  (Utilities|FlowControl|Delay 1.0)
  (Animation|Montage|PlayMontage (Actor|GetComponentbyClass _asboss_monster "/Script/Engine.SkeletalMeshComponent") "/Game/BossMonster/Characters/Characters/Heroes/Grux/Animations/LevelStart_Montage.LevelStart_Montage"
    (:OnCompleted
      (AI|RunBehaviorTree "/Game/BossMonster/Characters/Characters/Heroes/Grux/Boss_AI/BT_Boss.BT_Boss"))))

(fn ConstructionScript)