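; Player Blueprint that manages the in-game HUD, pause and game-over screens, and right-click targeting feedback.
; On possession it shows a PlayerHP widget unless the level matches Levelname, then Tick refreshes HP, command and skill text through UIcontroller.
; When IsDead is set, Tick pauses the game and shows GameOver.
; Escape toggles the pause widget, and right-click spawns a Niagara movement marker at the cursor hit without moving the player.
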(event EventPossessed
  (params (NewController :type Controller%20Object%20Reference))
  (bind _returnvalue (UserInterface|CreateWidget "/Game/Blueprints/Game_UI/PlayerHP.PlayerHP_C" (Game|GetPlayerController 0)))
  ;[1 1 1] UI생성관련
  (bind _returnvalue_2 (Game|GetCurrentLevelName true))
  (bind _output_get (Variables|Default|SetisMenu (Utilities|Enum|NotEqual(Enum) _returnvalue_2 (Variables|Default|Getlevelname))))
  (if _output_get
    (Variables|Default|SetUIwidget _returnvalue)
    (UserInterface|Viewport|AddtoViewport (Variables|Default|GetUIwidget) 0)
    (Utilities|FlowControl|Delay 0.05)
    (CallFunction|UIcontroller)))

(event EventTick
  (params (DeltaSeconds :type Float%20%28single-precision%29))
  (if (Variables|Default|GetisDead)
    (bind _returnvalue (UserInterface|CreateWidget "/Game/Blueprints/Game_UI/GameOver.GameOver_C" (Game|GetPlayerController 0)))
    (Game|SetGamePaused true)
    (UserInterface|Viewport|AddtoViewport _returnvalue 0)
    (elif (Variables|Default|GetisMenu)
      (CallFunction|UIcontroller))))

(event Input|KeyboardEvents|Escape
  (params (Key :type Key%20Structure :default "None"))
  (:Pressed
    (if (Variables|Default|GetisPaused)
      (Widget|RemovefromParent (stale _returnvalue))
      (Game|SetGamePaused false)
      (Variables|Default|SetisPaused false)
      (else
        (bind _returnvalue (UserInterface|CreateWidget "/Game/Blueprints/Game_UI/GamePause.GamePause_C" (Game|GetPlayerController 0)))
        (UserInterface|Viewport|AddtoViewport _returnvalue 0)
        (Game|SetGamePaused true)
        (Variables|Default|SetisPaused true)))))

(event Input|MouseEvents|RightMouseButton
  (params (Key :type Key%20Structure :default "None"))
  (bind _returnvalue (Game|GetPlayerController 0))
  (bind _trace_channel (Variables|Default|GetTrace%20Channel))
  (bind _hitresult (Game|Player|GetHitResultUnderCursorbyChannel _returnvalue _trace_channel false))
  (:Pressed
    (if (.bblockinghit _hitresult)
      (Niagara|SpawnSystematLocation "/Game/RPGEffects/ParticlesNiagara/TargetingDecals/NS_Targeting_Player_Movement.NS_Targeting_Player_Movement" (Math|Vector|MakeVector (.x (.location _hitresult)) (.y (.location _hitresult)) (+ (.z (.location _hitresult)) 0.1))))))

(fn ConstructionScript)

(fn UIcontroller
  (bind _uiwidget (Variables|Default|GetUIwidget))
  (Variables|/Game/Blueprints/Game_UI/PlayerHP.PlayerHP_C|SetHpRatio _uiwidget (/ (Math|Conversions|ToFloat(Integer) (Variables|Default|GetHP self)) (Math|Conversions|ToFloat(Integer) (Variables|Default|GetfullHP))))
  (Variables|/Game/Blueprints/Game_UI/PlayerHP.PlayerHP_C|SethpString _uiwidget (Utilities|String|Append (Utilities|String|ToString(Integer) (Variables|Default|GetHP)) "/" (Utilities|String|ToString(Integer) (Variables|Default|GetfullHP))))
  (Variables|/Game/Blueprints/Game_UI/PlayerHP.PlayerHP_C|SetcommandString _uiwidget (Variables|Default|GetcommandUI))
  (Variables|/Game/Blueprints/Game_UI/PlayerHP.PlayerHP_C|SetskillString _uiwidget (Variables|Default|GetSkillUI)))