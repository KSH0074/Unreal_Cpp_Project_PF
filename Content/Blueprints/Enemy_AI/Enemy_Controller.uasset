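; Enemy AI controller that runs the BT_Enemy behavior tree and feeds it blackboard state for player detection and distance from a starting point.
; On BeginPlay it records its own location as the initial point and stores the first player pawn.
; AI perception updates set a line-of-sight flag for successfully sensed Player-tagged actors and clear it otherwise.
; Each tick flags whether Me is at least TraceRange from that point.
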(event OnTargetPerceptionUpdated(AIPerception)
  (params (Actor :type Actor%20Object%20Reference) (Stimulus :type AI%20Stimulus%20Structure))
  (bind _blackboardcomp (Variables|Default|GetblackboardComp))
  (if (and (.bSuccessfullySensed (Utilities|Struct|BreakAIStimulus Stimulus)) (Actor|ActorHasTag Actor "Player"))
    (AI|Components|Blackboard|SetValueasBool _blackboardcomp (Variables|Default|GetHasLineOfSight) true)
    (else
      (AI|Components|Blackboard|SetValueasBool _blackboardcomp (Variables|Default|GetHasLineOfSight) false))))

(event EventBeginPlay
  (AI|RunBehaviorTree "/Game/Blueprints/Enemy_AI/BT_Enemy.BT_Enemy")
  (bind _output_get (Variables|Default|SetFirstLocation (Transformation|GetActorLocation)))
  (AI|Components|Blackboard|SetValueasVector (Variables|Default|GetblackboardComp) (Variables|Default|GetInitLocation) _output_get)
  (AI|Components|Blackboard|SetValueasObject (Variables|Default|GetblackboardComp) (Variables|Default|GetPlayerActor) (Game|Player|GetPlayerPawn 0)))

(event EventTick
  (params (DeltaSeconds :type Float%20%28single-precision%29))
  (bind _blackboardcomp (Variables|Default|GetblackboardComp))
  (if (>= (Math|Vector|Distance(Vector) (Transformation|GetActorLocation (Variables|Default|Getme)) (Variables|Default|GetFirstLocation)) (Variables|Default|GettraceRange))
    (AI|Components|Blackboard|SetValueasBool _blackboardcomp (Variables|Default|GetDistance) true)
    (else
      (AI|Components|Blackboard|SetValueasBool _blackboardcomp (Variables|Default|GetDistance) false))))

(fn ConstructionScript)